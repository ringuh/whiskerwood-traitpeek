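; BP_MapLoad is the map-load bootstrap for the TraitPeek mod, setting up its UI once the mod API reports loading finished.
; It adds a TraitLayer widget to the viewport, creates the TraitPeek widget, and passes it the layer root and a debug flag by property name.
; A non-empty debug.ini enables debug.
; Any key release adds TraitPeek to the viewport or, if already shown, resets its Waited and Bound state.
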(event `self.ReceiveBeginPlay`
  (add `ModAPI.onLoadingFinished` (`ModAPI.GetModAPI`) (delegate `OnLoaded`)))

(event `OnLoaded`
  (bind _returnvalue (`GameplayStatics.GetPlayerController` 0))
  (bind _returnvalue_2 (`ModAPI.ReadModTextFile` (`ModAPI.GetModAPI`) "TraitPeekConfig" "debug.ini"))
  (bind _output_get (set `self.Debug` (not (`KismetStringLibrary.IsEmpty` _returnvalue_2))))
  (bind _returnvalue_3 (`|CreateWidget` "/Game/Mods/TraitPeek/WBP_TraitLayer.WBP_TraitLayer_C" _returnvalue))
  (`UserWidget.AddToViewport` _returnvalue_3 5)
  (bind _returnvalue_4 (`|CreateWidget` "/Game/Mods/TraitPeek/WBP_TraitPeek.WBP_TraitPeek_C" _returnvalue))
  (set `self.Peek` _returnvalue_4)
  (`KismetSystemLibrary.SetObjectPropertyByName` _returnvalue_4 "LayerRoot" (`/Game/Mods/TraitPeek/WBP_TraitLayer.Root` _returnvalue_3))
  (`KismetSystemLibrary.SetBoolPropertyByName` _returnvalue_4 "Debug" _output_get)
  (`self.EnableInput` self _returnvalue)
  (if (`self.Debug`)
    (`ModAPI.LogMessage` (`ModAPI.GetModAPI`) "TraitPeek ready (1.1)" true)))

(event `Key|AnyKey` :consume false :paused true
  (params (Key :type "Key Structure"))
  (bind _peek (`self.Peek`))
  (:`Released`
    (if (`KismetSystemLibrary.IsValid` _peek)
      (if (`Widget.IsInViewport` _peek)
        (`KismetSystemLibrary.SetDoublePropertyByName` _peek "Waited")
        (`KismetSystemLibrary.SetBoolPropertyByName` _peek "Bound")
        (else
          (`UserWidget.AddToViewport` _peek 6))))))

(fn `UserConstructionScript`)